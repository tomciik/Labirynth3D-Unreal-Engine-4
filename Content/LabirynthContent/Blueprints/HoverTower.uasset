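; HoverTower is a component that flags its owning actor, presumably a tower, for highlighting while the cursor is over it.
; On BeginPlay it caches the owner's static mesh component and, if one exists, binds to the owner's begin and end cursor-over events.
; Those handlers toggle custom depth rendering on the mesh, the usual input for a post-process outline.
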(event `self.ReceiveBeginPlay`
  (bind _returnvalue (`self.GetOwner`))
  (bind _returnvalue_2 (`Actor.GetComponentByClass` _returnvalue "/Script/Engine.StaticMeshComponent"))
  (`/Engine/EditorBlueprintResources/StandardMacros.IsValid` _returnvalue_2
    (:`Is Valid`
      (set `self.StaticMesh` _returnvalue_2)
      (add `Actor.OnBeginCursorOver` _returnvalue (delegate `MouseHover`))
      (add `Actor.OnEndCursorOver` _returnvalue (delegate `MouseHoverOff`)))))

(event `MouseHover`
  (params (TouchedActor :type "Actor Object Reference"))
  (`PrimitiveComponent.SetRenderCustomDepth` (`self.StaticMesh`) true))

(event `MouseHoverOff`
  (params (TouchedActor :type "Actor Object Reference"))
  (`PrimitiveComponent.SetRenderCustomDepth` (`self.StaticMesh`) false))