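; LB_Controller is the Labyrinth controller that turns camera input actions into commands on the controlled LB_CameraControll_Snapping pawn.
; ChangeCamera toggles between side and overhead views, while the left and right rotation actions call the pawn's matching rotation functions.
; The toggle reads CameraOverhead from an instance found with GetActorOfClass, but every command goes to the controlled pawn through a cast.
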(event `InputAction|ChangeCamera`
  (params (Key :type "Key Structure"))
  (bind _returnvalue (`self.K2_GetPawn`))
  (:`Pressed`
    (bind _returnvalue_2 (`GameplayStatics.GetActorOfClass` "/Game/LabirynthContent/Blueprints/LB_CameraControll_Snapping.LB_CameraControll_Snapping_C"))
    (if (`/Game/LabirynthContent/Blueprints/LB_CameraControll_Snapping.CameraOverhead` _returnvalue_2)
      (bind _aslb_camera_controll_snapping (cast `/Game/LabirynthContent/Blueprints/LB_CameraControll_Snapping` _returnvalue))
      (`/Game/LabirynthContent/Blueprints/LB_CameraControll_Snapping.SideCamera` _aslb_camera_controll_snapping)
      (else
        (bind _aslb_camera_controll_snapping_2 (cast `/Game/LabirynthContent/Blueprints/LB_CameraControll_Snapping` _returnvalue))
        (`/Game/LabirynthContent/Blueprints/LB_CameraControll_Snapping.OverheadCamera` _aslb_camera_controll_snapping_2)))))

(event `InputAction|LeftRotationCamera`
  (params (Key :type "Key Structure"))
  (:`Pressed`
    (bind _aslb_camera_controll_snapping (cast `/Game/LabirynthContent/Blueprints/LB_CameraControll_Snapping` (`self.K2_GetPawn`)))
    (`/Game/LabirynthContent/Blueprints/LB_CameraControll_Snapping.LeftRotationCamera` _aslb_camera_controll_snapping)))

(event `InputAction|RightRotationCamera`
  (params (Key :type "Key Structure"))
  (:`Pressed`
    (bind _aslb_camera_controll_snapping (cast `/Game/LabirynthContent/Blueprints/LB_CameraControll_Snapping` (`self.K2_GetPawn`)))
    (`/Game/LabirynthContent/Blueprints/LB_CameraControll_Snapping.RightRotationCamera` _aslb_camera_controll_snapping)))

(fn `UserConstructionScript`)