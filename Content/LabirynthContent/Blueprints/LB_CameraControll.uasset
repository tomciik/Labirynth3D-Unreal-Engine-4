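; LB_CameraControll is a camera control Blueprint that rotates the view and handles tower placement.
; Left and right rotation events turn the SpringArm in quarter-turn steps.
; PlacementMode toggles placement, spawning a HitTower actor far below the world and destroying it when disabled.
; UpdatePlacement runs a debug-drawn line trace and moves that tower to any blocking hit, though nothing in this file calls it.
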(event `LeftRotationCamera`
  (`SceneComponent.K2_AddWorldRotation` (`self.SpringArm`) (struct :`Yaw` -90.0) false false))

(event `RightRotationCamera`
  (`SceneComponent.K2_AddWorldRotation` (`self.SpringArm`) (struct :`Yaw` 90.0) false false))

(fn `PlacementMode`
  (params (`Is Enabled` :type Boolean))
  (bind _hittower (`self.HitTower`))
  (if (== `Is Enabled` (`self.PlacementModeEnebled`))
    (return)
    (else
      (bind _output_get (set `self.PlacementModeEnebled` `Is Enabled`))
      (if _output_get
        (bind _returnvalue (`|SpawnActorFromClass` (`self.hitTowerClass`) (`KismetMathLibrary.MakeTransform` (0.0 0.0 -100000.0)) "Undefined" "OverrideRootScale" null null))
        (set `self.HitTower` _returnvalue)
        (`/Engine/EditorBlueprintResources/StandardMacros.IsValid` null)
        (else
          (`/Engine/EditorBlueprintResources/StandardMacros.IsValid` _hittower
            (:`Is Valid`
              (`self.K2_DestroyActor` _hittower))))))))

(fn `UpdatePlacement`
  (bind _outhit (`KismetSystemLibrary.LineTraceSingle` :`Start` (0.0 0.0 0.0) :`End` (+ (0.0 0.0 0.0) (* (0.0 0.0 0.0) 10000.0)) :`TraceChannel` "TraceTypeQuery3" :`bTraceComplex` true :`DrawDebugType` "ForDuration"))
  (bind (_bblockinghit _binitialoverlap _time _distance _location _impactpoint _normal _impactnormal _physmat _hitactor) (`GameplayStatics.BreakHitResult` _outhit))
  (if _bblockinghit
    (bind _output_get (set `self.HitTower` _hitactor))
    (`self.K2_SetActorLocation` _output_get _location false false)))

(fn `UserConstructionScript`)