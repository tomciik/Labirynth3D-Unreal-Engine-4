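; Labyrinth camera controller that switches between angled side and overhead views and lets the player place objects by snapping them.
; Spring-arm rotation sets the view, with 90-degree yaw steps in side view only.
; Overhead clicks toggle an object's held state, recolouring its post-process custom-depth highlight.
; While held, Tick traces from the cursor at the pick distance toward the object, snapping it to any detection box hit.
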(event `self.ReceiveBeginPlay`
  (set `self.CameraOverhead` false)
  (set `self.ClickedObject` false))

(event `SideCamera`
  ;[1 1 1] Camera change
  (`SceneComponent.K2_SetRelativeRotation` (`self.SpringArm`) (`KismetMathLibrary.MakeRotator` 0.0 -45.0 (`self.AngleZ`)) false false)
  (set `self.CameraOverhead` false)
  (set `self.ClickedObject` false))

(event `OverheadCamera`
  ;[1 1 1] Camera change
  (`SceneComponent.K2_SetRelativeRotation` (`self.SpringArm`) (`KismetMathLibrary.MakeRotator` 0.0 -90.0 (`self.AngleZ`)) false false)
  (set `self.CameraOverhead` true))

(event `LeftRotationCamera`
  (bind _springarm (`self.SpringArm`))
  (bind (_relativerotation_roll _relativerotation_pitch _relativerotation_yaw) (`KismetMathLibrary.BreakRotator` (`SceneComponent.RelativeRotation` _springarm)))
  ;[1 1 1] Camera rotation
  (if (not (`self.CameraOverhead`))
    (`SceneComponent.K2_AddRelativeRotation` _springarm (struct :`Yaw` 90.0) false false)
    (set `self.AngleZ` _relativerotation_yaw)))

(event `RightRotationCamera`
  (bind _springarm (`self.SpringArm`))
  (bind (_relativerotation_roll _relativerotation_pitch _relativerotation_yaw) (`KismetMathLibrary.BreakRotator` (`SceneComponent.RelativeRotation` _springarm)))
  ;[1 1 1] Camera rotation
  (if (not (`self.CameraOverhead`))
    (`SceneComponent.K2_AddRelativeRotation` _springarm (struct :`Yaw` -90.0) false false)
    (set `self.AngleZ` _relativerotation_yaw)))

(event `Key|LeftMouseButton`
  (params (Key :type "Key Structure"))
  (bind (_worldlocation _worlddirection) (`PlayerController.DeprojectMousePositionToWorld` (`GameplayStatics.GetPlayerController` 0)))
  (:`Pressed`
    (if (`self.CameraOverhead`)
      (bind (_outhit _returnvalue) (`KismetSystemLibrary.LineTraceSingle` :`Start` _worldlocation :`End` (+ _worldlocation (* _worlddirection 10000000.0)) :`TraceChannel` "TraceTypeQuery1" :`bTraceComplex` true :`DrawDebugType` "ForDuration"))
      (if _returnvalue
        (if (`self.ClickedObject`)
          (set `self.ClickedObject` false)
          (bind (_bblockinghit _binitialoverlap _time _distance _location _impactpoint _normal _impactnormal _physmat _hitactor) (`GameplayStatics.BreakHitResult` _outhit))
          (bind _returnvalue_2 (`self.GetComponentByClass` _hitactor "/Script/Engine.PostProcessComponent"))
          (set `PostProcessComponent.Settings` (`self.PostProcessSettings_green`) _returnvalue_2)
          (bind _returnvalue_3 (`self.GetComponentByClass` _hitactor "/Script/Engine.StaticMeshComponent"))
          (`PrimitiveComponent.SetRenderCustomDepth` _returnvalue_3 true)
          (else
            (set `self.ClickedObject` true)
            (set `self.OriginalDistance` _distance)
            (set `self.Object` _hitactor)
            (set `PostProcessComponent.Settings` (`self.PostProcessSettings_orange`) _returnvalue_2)
            (`PrimitiveComponent.SetRenderCustomDepth` _returnvalue_3 true)))))))

(event `self.ReceiveTick`
  (params (DeltaSeconds :type "Float (single-precision)"))
  (bind (_worldlocation _worlddirection) (`PlayerController.DeprojectMousePositionToWorld` (`GameplayStatics.GetPlayerController` 0)))
  (if (`self.CameraOverhead`)
    (if (`self.ClickedObject`)
      (`/Engine/EditorBlueprintResources/StandardMacros.IsValid` (`self.Object`)
        (:`Is Valid`
          (bind (_outhit _returnvalue) (`KismetSystemLibrary.LineTraceSingle` :`Start` (+ _worldlocation (* _worlddirection (`self.OriginalDistance`))) :`End` (`self.K2_GetActorLocation` (`self.Object`)) :`TraceChannel` "TraceTypeQuery2" :`bTraceComplex` true :`DrawDebugType` "ForDuration" :`DrawTime` 1.0))
          (if _returnvalue
            (bind (_bblockinghit _binitialoverlap _time _distance _location _impactpoint _normal _impactnormal _physmat _hitactor _hitcomponent) (`GameplayStatics.BreakHitResult` _outhit))
            (set `self.Hit Actor` _hitactor)
            (set `self.Hit Component` _hitcomponent)
            (bind (_found _transform) (`self.DetectionBoxes`))
            (if _found
              (`self.K2_SetActorTransform` (`self.Object`) (`KismetMathLibrary.MakeTransform` (.location _transform) (.rotation _transform)) false false))))))))

(fn `DetectionBoxes`
  (returns (Found :type Boolean) (Transform :type "Transform Structure"))
  (locals (LocalFound :type Boolean))
  (bind _newparam (message `/Game/LabirynthContent/Blueprints/Boxes.ReturnBox` (`self.Hit Actor`)))
  (for _array_element _newparam
    (if (== _array_element (`self.Hit Component`))
      (set `local.LocalFound` true)
      (break)))
  (return (`local.LocalFound`) (`SceneComponent.K2_GetComponentToWorld` (`self.Hit Component`))))

(fn `UserConstructionScript`)