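; Test camera Blueprint for the labyrinth content that switches between angled side and overhead views and lets the mouse move physics objects.
; View events set spring arm pitch and LB_Controller's CameraChange; both rotation events add 90° yaw in side view only.
; Overhead, a cursor trace grabs movable simulating components with a PhysicsHandle at their original distance.
; Tick traces toward the object and snaps it onto any hit detection box listed by ReturnBoxMessage.
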(event `self.ReceiveBeginPlay`
  ;[1 1 1] Camera change
  (bind _aslb_controller (cast `/Game/LabirynthContent/Blueprints/LB_Controller` (`GameplayStatics.GetPlayerController` 0)))
  (set `/Game/LabirynthContent/Blueprints/LB_Controller.CameraChange` true _aslb_controller)
  (set `self.CameraOverhead` false))

(event `SideCamera`
  ;[1 1 1] Camera change
  (`SceneComponent.K2_SetRelativeRotation` (`self.SpringArm`) (`KismetMathLibrary.MakeRotator` 0.0 -45.0 (`self.AngleZ`)) false false)
  (bind _aslb_controller (cast `/Game/LabirynthContent/Blueprints/LB_Controller` (`GameplayStatics.GetPlayerController` 0)))
  (set `/Game/LabirynthContent/Blueprints/LB_Controller.CameraChange` true _aslb_controller)
  (set `self.CameraOverhead` false)
  (`PhysicsHandleComponent.ReleaseComponent` (`self.PhysicsHandle`)))

(event `OverheadCamera`
  ;[1 1 1] Camera change
  (`SceneComponent.K2_SetRelativeRotation` (`self.SpringArm`) (`KismetMathLibrary.MakeRotator` 0.0 -90.0 (`self.AngleZ`)) false false)
  (bind _aslb_controller (cast `/Game/LabirynthContent/Blueprints/LB_Controller` (`GameplayStatics.GetPlayerController` 0)))
  (set `/Game/LabirynthContent/Blueprints/LB_Controller.CameraChange` false _aslb_controller)
  (set `self.CameraOverhead` true))

(event `LeftRotationCamera`
  (bind _springarm (`self.SpringArm`))
  (bind (_relativerotation_roll _relativerotation_pitch _relativerotation_yaw) (`KismetMathLibrary.BreakRotator` (`SceneComponent.RelativeRotation` _springarm)))
  ;[1 1 1] Camera rotation
  (if (not (`self.CameraOverhead`))
    (`SceneComponent.K2_AddRelativeRotation` _springarm (struct :`Yaw` 90.0) false false)
    (set `self.AngleZ` _relativerotation_yaw)))

(event `RightRotationCamera`
  (bind _springarm (`self.SpringArm`))
  (bind (_relativerotation_roll _relativerotation_pitch _relativerotation_yaw) (`KismetMathLibrary.BreakRotator` (`SceneComponent.RelativeRotation` _springarm)))
  ;[1 1 1] Camera rotation
  (if (not (`self.CameraOverhead`))
    (`SceneComponent.K2_AddRelativeRotation` _springarm (struct :`Yaw` 90.0) false false)
    (set `self.AngleZ` _relativerotation_yaw)))

(event `Key|LeftMouseButton`
  (params (Key :type "Key Structure"))
  (bind _grabbedobjects (`self.GrabbedObjects`))
  (bind (_worldlocation _worlddirection) (`PlayerController.DeprojectMousePositionToWorld` (`GameplayStatics.GetPlayerController` 0)))
  ;[1 1 1] LineTrace, grab and release objects
  (:`Pressed`
    (bind (_outhit _returnvalue) (`KismetSystemLibrary.LineTraceSingle` :`Start` _worldlocation :`End` (+ _worldlocation (* _worlddirection 10000000.0)) :`TraceChannel` "TraceTypeQuery1" :`bTraceComplex` true :`DrawDebugType` "ForDuration"))
    (if _returnvalue
      (if (`|EnumEquality` (`SceneComponent.Mobility` (`.HitComponent` (`GameplayStatics.BreakHitResult` _outhit))) (enumliteral `EComponentMobility` "Movable"))
        (bind (_bblockinghit _binitialoverlap _time _distance _location _impactpoint _normal _impactnormal _physmat _hitactor _hitcomponent) (`GameplayStatics.BreakHitResult` _outhit))
        (set `self.OriginalDistance` _distance)
        (bind _output_get (set `self.GrabbedObjects` _hitcomponent))
        (if (`SceneComponent.IsSimulatingPhysics` _output_get "None")
          (if (`self.CameraOverhead`)
            (`PhysicsHandleComponent.GrabComponentAtLocationWithRotation` (`self.PhysicsHandle`) _grabbedobjects "None" (`.Location` (`GameplayStatics.BreakHitResult` _outhit)) (`SceneComponent.K2_GetComponentRotation` _grabbedobjects)))))))
  (:`Released`
    (`PhysicsHandleComponent.ReleaseComponent` (`self.PhysicsHandle`))))

(event `self.ReceiveTick`
  (params (DeltaSeconds :type "Float (single-precision)"))
  (bind _grabbedobjects (`self.GrabbedObjects`))
  (bind (_worldlocation _worlddirection) (`PlayerController.DeprojectMousePositionToWorld` (`GameplayStatics.GetPlayerController` 0)))
  (bind _returnvalue (+ _worldlocation (* _worlddirection (`self.OriginalDistance`))))
  (if (`self.CameraOverhead`)
    (`/Engine/EditorBlueprintResources/StandardMacros.IsValid` _grabbedobjects
      (:`Is Valid`
        (if (`SceneComponent.IsSimulatingPhysics` _grabbedobjects "None")
          (`PhysicsHandleComponent.SetTargetLocation` (`self.PhysicsHandle`) _returnvalue)
          (bind (_outhit _returnvalue_2) (`KismetSystemLibrary.LineTraceSingle` :`Start` _returnvalue :`End` (`SceneComponent.K2_GetComponentLocation` (`self.GrabbedObjects`)) :`TraceChannel` "TraceTypeQuery1" :`DrawDebugType` "ForDuration" :`DrawTime` 1.0))
          (if _returnvalue_2
            (bind (_bblockinghit _binitialoverlap _time _distance _location _impactpoint _normal _impactnormal _physmat _hitactor _hitcomponent) (`GameplayStatics.BreakHitResult` _outhit))
            (set `self.Hit Actor` _hitactor)
            (set `self.Hit Component` _hitcomponent)
            (bind (_found _transform) (`self.DetectionBoxes`))
            (if _found
              (`SceneComponent.K2_SetWorldTransform` (`self.GrabbedObjects`) (`KismetMathLibrary.MakeTransform` (.location _transform) (.rotation _transform) (2.5 2.5 2.5)) false false))))))))

(fn `DetectionBoxes`
  (returns (Found :type Boolean) (Transform :type "Transform Structure"))
  (locals (LocalFound :type Boolean))
  (bind _newparam (message `/Game/LabirynthContent/Blueprints/Boxes.ReturnBox` (`self.Hit Actor`)))
  (for _array_element _newparam
    (if (== _array_element (`self.Hit Component`))
      (set `local.LocalFound` true)
      (break)))
  (return (`local.LocalFound`) (`SceneComponent.K2_GetComponentToWorld` (`self.Hit Component`))))

(fn `UserConstructionScript`)